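; BP_FloorTile is a self-replacing floor segment for an endless runner, with an attach transform for chaining tiles.
; When the player hits its end trigger, it asks the game mode to add a tile, then destroys itself after a delay; its kill floor triggers player death.
; Construction randomly adds blockers at left, middle or right spawn points, a coin within the item area, or nothing.
; Blocker placement and spawn-point removal roll separately, so blockers can share a point.
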(event `self.EndTrigger.OnComponentBeginOverlap`
  (params (OverlappedComponent :type "PrimitiveComponent Object Reference") (OtherActor :type "Actor Object Reference") (OtherComp :type "PrimitiveComponent Object Reference") (OtherBodyIndex :type Integer) (bFromSweep :type Boolean) (SweepResult :type "HitResult Structure (by ref)"))
  (cast `/Game/Blueprints/BP_ThirdPersonCharacter` OtherActor)
  (bind _asbp_third_person_game_mode (cast `/Game/Blueprints/BP_ThirdPersonGameMode` (`GameplayStatics.GetGameMode`)))
  (`/Game/Blueprints/BP_ThirdPersonGameMode.AddFloorTile` _asbp_third_person_game_mode)
  (`KismetSystemLibrary.Delay` 2.0)
  (`self.K2_DestroyActor`))

(event `self.KillFloor.OnComponentBeginOverlap`
  (params (OverlappedComponent :type "PrimitiveComponent Object Reference") (OtherActor :type "Actor Object Reference") (OtherComp :type "PrimitiveComponent Object Reference") (OtherBodyIndex :type Integer) (bFromSweep :type Boolean) (SweepResult :type "HitResult Structure (by ref)"))
  (bind _asbp_third_person_character (cast `/Game/Blueprints/BP_ThirdPersonCharacter` OtherActor))
  (`/Game/Blueprints/BP_ThirdPersonCharacter.death` _asbp_third_person_character))

(fn `GetAttachTransform`
  (returns (AttachTransform :type "Transform Structure"))
  (return (`SceneComponent.K2_GetComponentToWorld` (`self.AttachPoint`))))

(fn `SetSpawnPoints`
  (set `self.SpawnPoints` (`|MakeArray` (`SceneComponent.GetRelativeTransform` (`self.SpawnPointL`)) (`SceneComponent.GetRelativeTransform` (`self.SpawnPoint`)) (`SceneComponent.GetRelativeTransform` (`self.SpawnPointR`)))))

(fn `SpawnBlocker`
  (bind _spawnpoints (`self.SpawnPoints`))
  (bind _output (`|GetArrayItem` _spawnpoints (`KismetMathLibrary.RandomIntegerInRange` 0 (`KismetArrayLibrary.Array_LastIndex` _spawnpoints))))
  (for _ (range 2)
    (`AddComponent|NODE_AddChildActorComponent-0` :`RelativeTransform` _output)
    (`KismetArrayLibrary.Array_RemoveItem` _spawnpoints _output)))

(fn `SpawnCoins`
  (bind _itemarea (`self.ItemArea`))
  (`AddComponent|NODE_AddChildActorComponent-2` :`RelativeTransform` (`KismetMathLibrary.Conv_VectorToTransform` (`KismetMathLibrary.RandomPointInBoundingBox` (`SceneComponent.RelativeLocation` _itemarea) (`BoxComponent.BoxExtent` _itemarea)))))

(fn `UserConstructionScript`
  (`self.SetSpawnPoints`)
  (switch `int` (`KismetMathLibrary.RandomIntegerInRange` 0 3)
    (:`0`
      (`self.SpawnBlocker`))
    (:`1`
      (`self.SpawnCoins`))))